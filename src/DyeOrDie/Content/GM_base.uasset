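; GM_base is the game mode that runs enemy waves, score and loot drops.
; After an initial delay it passes the wave number to every BP_enemySpawner, then increments it.
; Pufferfish and octopus eliminations add score and decrement EnemiesLeft; at zero, the next wave spawns and the player heals.
; SpawnDrop makes a weighted random pick from the LoopOptions class-to-weight map, whose total is computed at BeginPlay, and prints debug values.
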(event `self.ReceiveBeginPlay`
  (`self.calculateLootOdds`)
  (`KismetSystemLibrary.Delay` (`self.intialSpawnDelay`))
  (`self.spawnEnemies`))

(event `spawnEnemies`
  (bind _wave (`self.wave`))
  (bind _outactors (`GameplayStatics.GetAllActorsOfClass` "/Game/Animals/BP_enemySpawner.BP_enemySpawner_C"))
  (for _array_element _outactors
    (`/Game/Animals/BP_enemySpawner.SpawnEnemies` _array_element _wave))
  (`/Engine/EditorBlueprintResources/StandardMacros.IncrementInt` _wave))

(event `checkSpawnEnemies`
  (if (== (`self.enemiesLeft`) 0)
    (`self.spawnEnemies`)
    (bind _asbp_blue_char (cast `/Game/Character/BP_blueChar` (`GameplayStatics.GetPlayerCharacter` 0)))
    (`/Game/Character/BP_blueChar.HealPlayer` _asbp_blue_char 15.0)))

(event `EliminatedPufferFish`
  (`/Engine/EditorBlueprintResources/StandardMacros.DecrementInt` (`self.enemiesLeft`)
    (:`  `
      (`/Engine/EditorBlueprintResources/StandardMacros.IncrementInt` (`self.score`)
        (:`  `
          (`self.checkSpawnEnemies`))))))

(event `EliminatedOctopus`
  (`/Engine/EditorBlueprintResources/StandardMacros.DecrementInt` (`self.enemiesLeft`)
    (:`  `
      (set `self.score` (+ (`self.score`) (`self.OctopusScorePoints`)))
      (`self.checkSpawnEnemies`))))

(fn `calculateLootOdds`
  (bind _values (`BlueprintMapLibrary.Map_Values` (`self.LoopOptions`)))
  (for _array_element _values
    (set `self.lootdropCounter` (+ _array_element (`self.lootdropCounter`)))))

(fn `spawnDrop`
  (params (location :type "Vector Structure"))
  (locals (dropValue :type Integer :default 0) (counter :type Integer))
  (set `local.dropValue` (`KismetMathLibrary.RandomInteger` (`self.lootdropCounter`)))
  (bind _values (`BlueprintMapLibrary.Map_Values` (`self.LoopOptions`)))
  (for (_array_element _array_index) _values
    (set `local.counter` (+ _array_element (`local.counter`)))
    (if (<= (`local.dropValue`) (`local.counter`))
      (bind _keys (`BlueprintMapLibrary.Map_Keys` (`self.LoopOptions`)))
      (`|SpawnActorFromClass` (`|GetArrayItem` _keys _array_index) (`KismetMathLibrary.MakeTransform` location) "AdjustIfPossibleButAlwaysSpawn" "OverrideRootScale" null null)
      (`KismetSystemLibrary.PrintString` (`KismetStringLibrary.Conv_IntToString` (`local.counter`)))
      (`KismetSystemLibrary.PrintString` (`KismetStringLibrary.Conv_IntToString` (`local.dropValue`)))
      (break))))

(fn `UserConstructionScript`)
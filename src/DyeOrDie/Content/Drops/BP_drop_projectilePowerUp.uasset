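; BP_drop_projectilePowerUp is a pawn pickup that reduces the player character's projectile cooldown when collected.
; While BP_blueChar is inside the SearchSphere, Tick issues AIMoveTo toward the player, and leaving the sphere stops movement immediately.
; Overlapping the CollectSphere calls ReduceProjectileCooldown with DelayReduction and destroys the drop.
; If never collected, it destroys itself after DestroySelfDelay.
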(event `self.ReceiveBeginPlay`
  (bind _asbp_blue_char (cast `/Game/Character/BP_blueChar` (`GameplayStatics.GetPlayerCharacter` 0)))
  (set `self.playerRef` _asbp_blue_char)
  (`KismetSystemLibrary.Delay` (`self.destroySelfDelay`))
  (`self.K2_DestroyActor`))

(event `self.ReceiveTick`
  (params (DeltaSeconds :type "Float (single-precision)"))
  (if (`self.searchingForPlayer`)
    (`|AIMoveTo` self (0.0 0.0 0.0) (`self.playerRef`) 20.0)))

(event `self.SearchSphere.OnComponentBeginOverlap`
  (params (OverlappedComponent :type "PrimitiveComponent Object Reference") (OtherActor :type "Actor Object Reference") (OtherComp :type "PrimitiveComponent Object Reference") (OtherBodyIndex :type Integer) (bFromSweep :type Boolean) (SweepResult :type "HitResult Structure (by ref)"))
  (cast `/Game/Character/BP_blueChar` OtherActor)
  (set `self.searchingForPlayer` true))

(event `self.SearchSphere.OnComponentEndOverlap`
  (params (OverlappedComponent :type "PrimitiveComponent Object Reference") (OtherActor :type "Actor Object Reference") (OtherComp :type "PrimitiveComponent Object Reference") (OtherBodyIndex :type Integer))
  (cast `/Game/Character/BP_blueChar` OtherActor)
  (set `self.searchingForPlayer` false)
  (`MovementComponent.StopMovementImmediately` (`self.FloatingPawnMovement`)))

(event `self.CollectSphere.OnComponentBeginOverlap`
  (params (OverlappedComponent :type "PrimitiveComponent Object Reference") (OtherActor :type "Actor Object Reference") (OtherComp :type "PrimitiveComponent Object Reference") (OtherBodyIndex :type Integer) (bFromSweep :type Boolean) (SweepResult :type "HitResult Structure (by ref)"))
  (bind _asbp_blue_char (cast `/Game/Character/BP_blueChar` OtherActor))
  (`/Game/Character/BP_blueChar.reduceProjectileCooldown` _asbp_blue_char (`self.delayReduction`))
  (`self.K2_DestroyActor`))

(fn `UserConstructionScript`)
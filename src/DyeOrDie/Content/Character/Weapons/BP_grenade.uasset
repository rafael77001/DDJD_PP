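; BP_grenade is a thrown-weapon actor that explodes on impact and kills nearby puffer fish.
; Half a second after BeginPlay it sets its sphere to block all channels and arms itself.
; On an armed hit it spawns an actor scaled in X and Z by Radius, apparently an explosion sprite.
; It then calls Die on every BP_pufferFish within Radius via a distance check and destroys itself.
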(event `self.ReceiveBeginPlay`
  (`KismetSystemLibrary.Delay` 0.5)
  (`PrimitiveComponent.SetCollisionResponseToAllChannels` (`self.grenade sphere`) "ECR_Block")
  (set `self.active` true))

(event `self.grenade sphere.OnComponentHit`
  (params (HitComponent :type "PrimitiveComponent Object Reference") (OtherActor :type "Actor Object Reference") (OtherComp :type "PrimitiveComponent Object Reference") (NormalImpulse :type "Vector Structure") (Hit :type "HitResult Structure (by ref)"))
  (bind _returnvalue (/ (`self.radius`) (`self.explosionSpriteReducer`)))
  (if (`self.active`)
    (`|SpawnActorFromClass` "/Game/Character/Weapons/BP_bombExplosion.BP_bombExplosion_C" (`KismetMathLibrary.MakeTransform` (`self.K2_GetActorLocation`) (struct) (`KismetMathLibrary.MakeVector` _returnvalue 0.0 _returnvalue)) "Undefined" "OverrideRootScale" null null)
    (bind _outactors (`GameplayStatics.GetAllActorsOfClass` "/Game/Animals/fish2D/BP_pufferFish.BP_pufferFish_C"))
    (for _array_element _outactors
      (if (< (`KismetMathLibrary.Vector_Distance` (`self.K2_GetActorLocation`) (`self.K2_GetActorLocation` _array_element)) (`self.radius`))
        (`KismetSystemLibrary.PrintString` "destroyed puffer fish")
        (`/Game/Animals/fish2D/BP_pufferFish.Die` _array_element)))
    (`self.K2_DestroyActor`)))

(fn `UserConstructionScript`)
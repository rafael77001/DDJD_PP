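; BP_Projectile is a weapon projectile that kills BP_pufferFish on impact.
; It arms itself shortly after spawning by setting its sphere to block all collision channels and marking itself active.
; Once active, a hit calls Die on a matching pufferfish, and the projectile destroys itself, as it does when hitting anything else.
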(event `self.ReceiveBeginPlay`
  (`KismetSystemLibrary.Delay` 0.2)
  (`PrimitiveComponent.SetCollisionResponseToAllChannels` (`self.projectileSphere`) "ECR_Block")
  (set `self.active` true))

(event `self.projectileSphere.OnComponentHit`
  (params (HitComponent :type "PrimitiveComponent Object Reference") (OtherActor :type "Actor Object Reference") (OtherComp :type "PrimitiveComponent Object Reference") (NormalImpulse :type "Vector Structure") (Hit :type "HitResult Structure (by ref)"))
  (if (`self.active`)
    (if (== OtherActor "/Game/Animals/fish2D/BP_pufferFish.BP_pufferFish_C")
      (bind _asbp_puffer_fish (cast `/Game/Animals/fish2D/BP_pufferFish` OtherActor))
      (`/Game/Animals/fish2D/BP_pufferFish.Die` _asbp_puffer_fish))
    (`self.K2_DestroyActor`)))

(fn `UserConstructionScript`)
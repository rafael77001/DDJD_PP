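; Player character Blueprint with Enhanced Input movement, mouse-aimed shooting and grenade throwing, and a health system.
; BeginPlay adds input mappings, shows the cursor, creates HUD widgets and makes a dynamic sprite material.
; Left-click release fires the toggled weapon along the deprojected cursor direction, gated by per-weapon delays.
; Damage and healing flash the sprite through timelines; death shows game over and pauses.
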(event `EnhancedInput|/Game/Character/input/IA_switchWeapons`
  (params (ActionValue :type Boolean) (ElapsedSeconds :type "Float (double-precision)") (TriggeredSeconds :type "Float (double-precision)") (InputAction :type "InputAction Object Reference" :default "/Game/Character/input/IA_switchWeapons.IA_switchWeapons"))
  (:`Started`
    (if (`self.grenadeEquiped`)
      (set `self.grenadeEquiped` false)
      (else
        (set `self.grenadeEquiped` true)))))

(event `EnhancedInput|/Game/Character/input/inputAction_move`
  (params (ActionValue :type "Vector2D Structure") (ElapsedSeconds :type "Float (double-precision)") (TriggeredSeconds :type "Float (double-precision)") (InputAction :type "InputAction Object Reference" :default "/Game/Character/input/inputAction_move.inputAction_move"))
  (:`Triggered`
    (`self.AddMovementInput` (1.0 0.0 0.0) ActionValue_X)
    (`self.AddMovementInput` (0.0 -1.0 0.0) ActionValue_Y)
    (set `self.Directionality` (`KismetMathLibrary.MakeVector2D` ActionValue_X ActionValue_Y)))
  (:`Started`
    (set `self.isHoldingMoveKey` true))
  (:`Completed`
    (set `self.isHoldingMoveKey` false)))

(event `self.ReceiveBeginPlay`
  (`|ExecutionSequence`
    (:`then_0`
      (bind _asplayer_controller (cast `PlayerController` (`self.GetController`)))
      (bind _returnvalue (pcsubsystem `EnhancedInputLocalPlayerSubsystem` _asplayer_controller))
      (`EnhancedInputSubsystemInterface.AddMappingContext` _returnvalue "/Game/Character/input/IMC_move.IMC_move" 0 (struct))
      (`EnhancedInputSubsystemInterface.AddMappingContext` _returnvalue "/Game/Character/input/IMC_characterActions.IMC_characterActions" 0 (struct)))
    (:`then_1`
      (set `PlayerController.bShowMouseCursor` true (`GameplayStatics.GetPlayerController` 0))
      (bind _returnvalue_2 (`|CreateWidget` "/Game/UI/WD_healthBar.WD_healthBar_C"))
      (`UserWidget.AddToViewport` _returnvalue_2 0)
      (bind _returnvalue_3 (`|CreateWidget` "/Game/UI/WD_score.WD_score_C"))
      (`UserWidget.AddToViewport` _returnvalue_3 0)
      (bind _returnvalue_4 (`|CreateWidget` "/Game/UI/WD_weaponEquipped.WD_weaponEquipped_C"))
      (`UserWidget.AddToViewport` _returnvalue_4 0))
    (:`then_2`
      (bind _returnvalue_5 (`PrimitiveComponent.CreateDynamicMaterialInstance` (`self.Sprite`) 0 null "None"))
      (set `self.dynamicSpriteMaterial` _returnvalue_5))))

(event `Key|LeftMouseButton`
  (params (Key :type "Key Structure"))
  (:`Released`
    (if (`self.grenadeEquiped`)
      (if (`self.CanThrowGrenade`)
        (`self.ThrowGrenade`)
        (set `self.CanThrowGrenade` false)
        (`KismetSystemLibrary.Delay` (`self.throwGrenadeDelay`))
        (set `self.CanThrowGrenade` true))
      (elif (`self.canShoot`)
        (`self.shootProjectile`)
        (set `self.canShoot` false)
        (`KismetSystemLibrary.Delay` (`self.shootingDelay`))
        (set `self.canShoot` true)))))

(event `DamagePlayer`
  (params (damage :type "Float (double-precision)" :default 45.0))
  (set `self.health` (- (`self.health`) damage))
  (`self.CheckDied`)
  (`MaterialInstanceDynamic.SetVectorParameterValue` (`self.dynamicSpriteMaterial`) "FlashColor" (struct :`G` 0.8 :`B` 0.639216 :`A` 1.0))
  (bind (_direction _alpha) (`Timeline|FlashMultiplier` :!via `PlayFromStart`)
    (:`Update`
      (`MaterialInstanceDynamic.SetScalarParameterValue` (`self.dynamicSpriteMaterial`) "FlashMultiplier" (`KismetMathLibrary.Lerp` 0.0 1.0 _alpha)))))

(event `HealPlayer`
  (params (HealAmount :type "Float (double-precision)" :default 15.0))
  (bind _returnvalue (+ HealAmount (`self.health`)))
  (if (> _returnvalue (`self.maxHealth`))
    (set `self.health` (`self.maxHealth`))
    (else
      (set `self.health` _returnvalue)))
  (`MaterialInstanceDynamic.SetVectorParameterValue` (`self.dynamicSpriteMaterial`) "FlashColor" (struct :`R` 0.486275 :`G` 0.054902 :`B` 0.701961 :`A` 1.0))
  (bind (_direction _alpha) (`Timeline|Timeline` :!via `PlayFromStart`)
    (:`Update`
      (`MaterialInstanceDynamic.SetScalarParameterValue` (`self.dynamicSpriteMaterial`) "FlashMultiplier" (`KismetMathLibrary.Lerp` 0.0 1.0 _alpha)))))

(fn `CheckDied`
  (if (<= (`self.health`) 0.0)
    (bind _returnvalue (`|CreateWidget` "/Game/UI/WD_gameOver.WD_gameOver_C"))
    (`UserWidget.AddToViewport` _returnvalue 0)
    (`GameplayStatics.SetGamePaused` true)))

(fn `IncreaseMaxHealth`
  (params (maxHealthAmount :type "Float (double-precision)"))
  (set `self.maxHealth` (+ (`self.maxHealth`) maxHealthAmount))
  (`self.HealPlayer` maxHealthAmount))

(fn `shootProjectile`
  (bind _projectilespeed (`self.projectileSpeed`))
  (bind (_worldlocation _worlddirection) (`PlayerController.DeprojectMousePositionToWorld` (`GameplayStatics.GetPlayerController` 0)))
  (bind (_worldlocation_2 _worlddirection_2) (`PlayerController.DeprojectMousePositionToWorld` (`GameplayStatics.GetPlayerController` 0)))
  (bind _returnvalue (`|SpawnActorFromClass` "/Game/Character/Weapons/BP_Projectile.BP_Projectile_C" (`KismetMathLibrary.MakeTransform` (`SceneComponent.K2_GetComponentLocation` (`self.spawnProjectileRef`)) (`KismetMathLibrary.Conv_VectorToRotator` (`KismetMathLibrary.Normal` (`KismetMathLibrary.MakeVector` (.x _worlddirection_2) (.y _worlddirection_2))))) "AlwaysSpawn" "OverrideRootScale" null null))
  (set `MovementComponent.Velocity` (`KismetMathLibrary.MakeVector` (* (.x _worlddirection) _projectilespeed) (* _projectilespeed (.y _worlddirection)) (+ (.z _worlddirection) 150.0)) (`/Game/Character/Weapons/BP_Projectile.ProjectileMovement` _returnvalue)))

(fn `ThrowGrenade`
  (bind _grenadespeed (`self.grenadeSpeed`))
  (bind (_worldlocation _worlddirection) (`PlayerController.DeprojectMousePositionToWorld` (`GameplayStatics.GetPlayerController` 0)))
  (bind _returnvalue (`|SpawnActorFromClass` "/Game/Character/Weapons/BP_grenade.BP_grenade_C" (`KismetMathLibrary.MakeTransform` (`SceneComponent.K2_GetComponentLocation` (`self.spawnProjectileRef`))) "AlwaysSpawn" "OverrideRootScale" null null))
  (set `MovementComponent.Velocity` (`KismetMathLibrary.MakeVector` (* (.x _worlddirection) _grenadespeed) (* _grenadespeed (.y _worlddirection)) (+ (.z _worlddirection) 150.0)) (`/Game/Character/Weapons/BP_grenade.ProjectileMovement` _returnvalue)))

(fn `UserConstructionScript`)
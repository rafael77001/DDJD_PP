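; BP_OctopusProjectile is a projectile actor, filed with the 2D fish animals, that damages the BP_blueChar player on impact.
; After a short delay on BeginPlay it sets its collision sphere to block all channels and marks itself active.
; Once active, any hit destroys it, calling DamagePlayer with its Damage value first if the other actor is BP_blueChar.
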(event `self.ReceiveBeginPlay`
  (`KismetSystemLibrary.Delay` 0.2)
  (`PrimitiveComponent.SetCollisionResponseToAllChannels` (`self.projectileSphere`) "ECR_Block")
  (set `self.active` true))

(event `self.projectileSphere.OnComponentHit`
  (params (HitComponent :type "PrimitiveComponent Object Reference") (OtherActor :type "Actor Object Reference") (OtherComp :type "PrimitiveComponent Object Reference") (NormalImpulse :type "Vector Structure") (Hit :type "HitResult Structure (by ref)"))
  (if (`self.active`)
    (if (== OtherActor "/Game/Character/BP_blueChar.BP_blueChar_C")
      (bind _asbp_blue_char (cast `/Game/Character/BP_blueChar` OtherActor))
      (`/Game/Character/BP_blueChar.DamagePlayer` _asbp_blue_char (`self.damage`)))
    (`self.K2_DestroyActor`)))

(fn `UserConstructionScript`)
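; Octopus enemy that chases the player, fires projectiles and dies on its own after a set delay.
; Tick uses AIMoveTo to reach shooting radius, then ShootProjectile launches a damage-carrying projectile toward the player with slight upward velocity, followed by a cooldown.
; Die stops movement and fades in a purple sprite flash via timeline and dynamic material, then reports to GM_base, spawns a drop and destroys the actor.
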(event `self.ReceiveBeginPlay`
  (bind _returnvalue (`PrimitiveComponent.CreateDynamicMaterialInstance` (`self.Sprite`) 0 null "None"))
  (set `self.DynamicSpriteMaterial` _returnvalue)
  (bind _asbp_blue_char (cast `/Game/Character/BP_blueChar` (`GameplayStatics.GetPlayerCharacter` 0)))
  (set `self.playerRef` _asbp_blue_char)
  (bind _asgm_base (cast `/Game/GM_base` (`GameplayStatics.GetGameMode`)))
  (`/Engine/EditorBlueprintResources/StandardMacros.IncrementInt` (`/Game/GM_base.enemiesLeft` _asgm_base)
    (:`  `
      (`KismetSystemLibrary.Delay` (`self.suicideDelay`))
      (`self.Die`))))

(event `self.ReceiveTick`
  (params (DeltaSeconds :type "Float (single-precision)"))
  (if (`self.canshoot`)
    (if (`self.Shooting`)
      (`self.ShootProjectile`)
      (set `self.canshoot` false)
      (`KismetSystemLibrary.Delay` (`self.ShootingDelay`))
      (set `self.Shooting` false)
      (set `self.canshoot` true)
      (else
        (`|AIMoveTo` self (`self.K2_GetActorLocation` (`self.playerRef`)) null (`self.shootingRadius`)
          (:`OnSuccess`
            (set `self.Shooting` true)))))))

(event `Die`
  (set `self.canshoot` false)
  (`Controller.StopMovement` (`AIBlueprintHelperLibrary.GetAIController` self))
  (`PrimitiveComponent.SetCollisionResponseToChannel` (`self.CapsuleComponent`) "ECC_PhysicsBody" "ECR_Overlap")
  (`MaterialInstanceDynamic.SetVectorParameterValue` (`self.dynamicSpriteMaterial`) "FlashColor" (struct :`R` 0.486275 :`G` 0.054902 :`B` 0.701961 :`A` 1.0))
  (bind (_direction _alpha) (`Timeline|Timeline`)
    (:`Update`
      (`MaterialInstanceDynamic.SetScalarParameterValue` (`self.dynamicSpriteMaterial`) "FlashMultiplier" (`KismetMathLibrary.Lerp` 0.0 1.0 _alpha)))
    (:`Finished`
      (bind _asgm_base (cast `/Game/GM_base` (`GameplayStatics.GetGameMode`)))
      (`/Game/GM_base.EliminatedOctopus` _asgm_base)
      (`/Game/GM_base.spawnDrop` _asgm_base (`self.K2_GetActorLocation`))
      (`self.K2_DestroyActor`))))

(fn `ShootProjectile`
  (bind _projectilespeed (`self.projectileSpeed`))
  (bind (_returnvalue_x _returnvalue_y _returnvalue_z) (`KismetMathLibrary.BreakVector` (`KismetMathLibrary.GetDirectionUnitVector` (`self.K2_GetActorLocation`) (`self.K2_GetActorLocation` (`self.playerRef`)))))
  (bind (_returnvalue_x_2 _returnvalue_y_2) (`KismetMathLibrary.BreakVector` (`KismetMathLibrary.GetDirectionUnitVector` (`self.K2_GetActorLocation`) (`self.K2_GetActorLocation` (`self.playerRef`)))))
  (if (`self.canshoot`)
    (bind _returnvalue (`|SpawnActorFromClass` "/Game/Animals/fish2D/BP_OctopusProjectile.BP_OctopusProjectile_C" (`KismetMathLibrary.MakeTransform` (`self.K2_GetActorLocation`) (`KismetMathLibrary.Conv_VectorToRotator` (`KismetMathLibrary.Normal` (`KismetMathLibrary.MakeVector` _returnvalue_x_2 _returnvalue_y_2)))) "AlwaysSpawn" "OverrideRootScale" null null))
    (set `/Game/Animals/fish2D/BP_OctopusProjectile.damage` (`self.Damage`) _returnvalue)
    (set `MovementComponent.Velocity` (`KismetMathLibrary.MakeVector` (* _returnvalue_x _projectilespeed) (* _projectilespeed _returnvalue_y) (+ _returnvalue_z 150.0)) (`/Game/Animals/fish2D/BP_OctopusProjectile.ProjectileMovement` _returnvalue))))

(fn `UserConstructionScript`)
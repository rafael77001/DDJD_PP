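; Pufferfish enemy that chases the player character and, on reaching it, acts as a delayed proximity bomb.
; Tick issues AI MoveTo toward the player until it succeeds, then Die stops movement, sets the capsule to overlap physics bodies and waits out a delay.
; It then damages BP_blueChar if still within the damage radius, reports the elimination to GM_base, spawns a drop and destroys itself.
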(event `self.ReceiveBeginPlay`
  (set `self.Player` (`GameplayStatics.GetPlayerCharacter` 0))
  (bind _asgm_base (cast `/Game/GM_base` (`GameplayStatics.GetGameMode`)))
  (`/Engine/EditorBlueprintResources/StandardMacros.IncrementInt` (`/Game/GM_base.enemiesLeft` _asgm_base)))

(event `self.ReceiveTick`
  (params (DeltaSeconds :type "Float (single-precision)"))
  (if (`self.Collided`)
    (`self.Die`)
    (else
      (`|AIMoveTo` self (0.0 0.0 0.0) (`self.Player`) (`self.hitRadius`)
        (:`OnSuccess`
          (set `self.Collided` true))))))

(event `Die`
  (set `self.Collided` true)
  (`Controller.StopMovement` (`AIBlueprintHelperLibrary.GetAIController` self))
  (`PrimitiveComponent.SetCollisionResponseToChannel` (`self.CapsuleComponent`) "ECC_PhysicsBody" "ECR_Overlap")
  (`KismetSystemLibrary.Delay` (`self.Damage Delay`))
  (`self.AfterCollision&Delay`))

(fn `AfterCollision&Delay`
  (bind _asbp_blue_char (cast `/Game/Character/BP_blueChar` (`self.Player`)))
  (if (not (>= (`KismetMathLibrary.Vector_Distance` (`self.K2_GetActorLocation` _asbp_blue_char) (`self.K2_GetActorLocation`)) (`self.DamageRadius`)))
    (`/Game/Character/BP_blueChar.DamagePlayer` _asbp_blue_char (`self.Damage`)))
  (bind _asgm_base (cast `/Game/GM_base` (`GameplayStatics.GetGameMode`)))
  (`/Game/GM_base.EliminatedPufferFish` _asgm_base)
  (`/Game/GM_base.spawnDrop` _asgm_base (`self.K2_GetActorLocation`))
  (`self.K2_DestroyActor`))

(fn `UserConstructionScript`)